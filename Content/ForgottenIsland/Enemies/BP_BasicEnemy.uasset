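; BP_BasicEnemy is a basic enemy Blueprint with a timer-driven sword trace for melee attacks.
; Attack starts a fast looping timer that fires StartTrace, and StopTrace clears it through the stored handle.
; Each StartTrace runs a Visibility line trace between two SwordMesh sockets with timed debug drawing, but the hit result is not yet used.
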(event `Attack`
  (bind _returnvalue (`KismetSystemLibrary.K2_SetTimerDelegate` (delegate `StartTrace`) 0.01 true))
  (set `self.TimeHandler` _returnvalue))

(event `StartTrace`
  (bind _sword_mesh (`self.Sword Mesh`))
  (`KismetSystemLibrary.LineTraceSingle` :`Start` (`SceneComponent.GetSocketLocation` _sword_mesh "StartTrace") :`End` (`SceneComponent.GetSocketLocation` _sword_mesh "EndTrace") :`TraceChannel` "TraceTypeQuery1" :`DrawDebugType` "ForDuration" :`DrawTime` 1.0))

(event `StopTrace`
  (`KismetSystemLibrary.K2_ClearAndInvalidateTimerHandle` (`self.TimeHandler`)))

(fn `UserConstructionScript`
  (`parent.UserConstructionScript`))