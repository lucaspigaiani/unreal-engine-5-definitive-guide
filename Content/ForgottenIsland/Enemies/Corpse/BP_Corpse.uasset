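; BP_Corpse is an enemy corpse character that damages the player with sword attacks.
; Attack starts a fast looping timer that line-traces between two sword sockets until StopTrace clears it.
; A hit player is damaged, then stored and ignored by later traces until StopTrace resets it, limiting each swing to one hit.
; On possession it binds a death event that silences its zombie sound and plays falling bones.
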(event `Attack`
  (bind _returnvalue (`KismetSystemLibrary.K2_SetTimerDelegate` (delegate `StartTrace`) 0.01 true))
  (set `self.TimeHandler` _returnvalue))

(event `StartTrace`
  (bind _sword_mesh (`self.Sword Mesh`))
  (bind _outhit (`KismetSystemLibrary.LineTraceSingle` (`SceneComponent.GetSocketLocation` _sword_mesh "StartTrace") (`SceneComponent.GetSocketLocation` _sword_mesh "EndTrace") "TraceTypeQuery1" false (`|MakeArray` (`self.Player`)) "None" true (struct :`R` 1.0 :`A` 1.0) (struct :`G` 1.0 :`A` 1.0) 1.0))
  (bind (_bblockinghit _binitialoverlap _time _distance _location _impactpoint _normal _impactnormal _physmat _hitactor) (`GameplayStatics.BreakHitResult` _outhit))
  (if (== (`GameplayStatics.GetObjectClass` _hitactor) "/Game/ForgottenIsland/Player/BP_Player.BP_Player_C")
    (bind _output_get (set `self.Player` _hitactor))
    (`GameplayStatics.ApplyDamage` _output_get 1.0)))

(event `StopTrace`
  (`KismetSystemLibrary.K2_ClearAndInvalidateTimerHandle` (`self.TimeHandler`))
  (set `self.Player` null))

(event `self.ReceivePossessed`
  (params (NewController :type "Controller Object Reference"))
  (add `self.Death` (delegate `DeathEvent`)))

(event `DeathEvent`
  ; Death event
  (`ActorComponent.SetActive` (`self.Zombie SFX`) false false)
  (`GameplayStatics.PlaySoundAtLocation` "/Game/ForgottenIsland/Enemies/Sounds/fallingBones_Cue.fallingBones_Cue" (`self.K2_GetActorLocation`) (struct) 0.7 1.0 0.0 null null null null))

(fn `UserConstructionScript`
  (`parent.UserConstructionScript`))