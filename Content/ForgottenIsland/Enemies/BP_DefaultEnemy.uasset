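; Base enemy character for Forgotten Island that takes damage, dies as a ragdoll and then removes itself.
; AnyDamage subtracts from Health within zero and MaxHealth, prints the result and, at zero, sets IsDead to ignore further hits.
; Death runs Ragdoll, which switches the mesh to physics and disables capsule collision and movement, then fires the Death dispatcher and destroys the actor after a short delay.
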(event `self.ReceiveAnyDamage`
  (params (Damage :type "Float (single-precision)") (DamageType :type "DamageType Object Reference") (InstigatedBy :type "Controller Object Reference") (DamageCauser :type "Actor Object Reference"))
  (if (not (`self.IsDead`))
    (bind _output_get (set `self.Health` (`KismetMathLibrary.FClamp` (- (`self.Health`) Damage) 0.0 (`self.MaxHealth`))))
    (`KismetSystemLibrary.PrintString` (`KismetStringLibrary.Conv_DoubleToString` _output_get))
    (if (== _output_get 0.0)
      (set `self.IsDead` true)
      (`self.Ragdoll`)
      (`self.Death`)
      (`KismetSystemLibrary.Delay` 5.0)
      (`self.K2_DestroyActor`))))

(event `Ragdoll`
  (`PrimitiveComponent.SetCollisionEnabled` (`self.CapsuleComponent`) "NoCollision")
  (`PrimitiveComponent.SetCollisionEnabled` (`self.Mesh`) "PhysicsOnly")
  (`PrimitiveComponent.SetSimulatePhysics` (`self.Mesh`) true)
  (`MovementComponent.StopMovementImmediately` (`self.CharacterMovement`))
  (`CharacterMovementComponent.DisableMovement` (`self.CharacterMovement`)))

(fn `UserConstructionScript`)